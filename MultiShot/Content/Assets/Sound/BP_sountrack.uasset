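; Soundtrack actor that plays looping background music from BeginPlay until a switch to a second track.
; BodyLocal spawns the Soundtrackloop sound attached to the root, stores it, and re-triggers itself after a 30-second delay while Condition is true.
; The SUPER event clears Condition, stops the most recently stored sound and plays SoundtrackBODY as 2D audio.
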(event Custom|body
  (CallFunction|BodyLocal))

(event Custom|BodyLocal
  (bind _returnvalue (Audio|SpawnSoundAttached "/Game/Assets/Sound/soundtrackloop.soundtrackloop" (Variables|Default|GetDefaultSceneRoot) "None" "0, 0, 0" "0, 0, 0" "KeepRelativeOffset" false 0.8 1.0 0.0 0 0))
  (Variables|Default|Setsound _returnvalue)
  (Utilities|FlowControl|Delay 3e+01)
  (if (Variables|Default|GetCondition)
    (CallFunction|BodyLocal)))

(event Custom|SUPER
  (CallFunction|Superlocal))

(event Custom|superlocal
  (Variables|Default|SetCondition false)
  (Audio|Components|Audio|Stop (Variables|Default|Getsound))
  (Audio|PlaySound2D "/Game/Assets/Sound/soundtrackBODY.soundtrackBODY" 1.5 1.0 0.0 0 0))

(event EventBeginPlay
  (CallFunction|Body))

(event Collision|EventActorBeginOverlap
  (params (OtherActor :type Actor%20Object%20Reference)))

(event EventTick
  (params (DeltaSeconds :type Float%20%28single-precision%29)))

(fn ConstructionScript)