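; BP_RandomSoundAmbient is an ambient sound actor that plays a sound effect repeatedly at random intervals from varying spots.
; After BeginPlay it waits a randomized delay around the Teimpo interval, then the Sonido event calls itself in an endless loop.
; Each play picks one of five scene component locations at random and applies randomized volume and lowered pitch with cave attenuation.
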(event Custom|Sonido
  (bind _teimpo (Variables|Default|GetTeimpo))
  (Audio|PlaySoundatLocation (Variables|Default|GetSFX) (Transformation|GetWorldLocation (.OutItem (Utilities|Array|Random (Utilities|Array|MakeArray (Variables|Default|GetScene3) (Variables|Default|GetScene2) (Variables|Default|GetScene1) (Variables|Default|GetScene) (Variables|Default|GetScene4))))) "0, 0, 0" (Math|Random|RandomFloatinRange 1.0 1.5) (Math|Random|RandomFloatinRange 0.7 0.9) 0.0 "/Game/VRE/Core/Character/CaveAtten.CaveAtten" 0 0 0)
  (Utilities|FlowControl|Delay (Math|Random|RandomFloatinRange (- _teimpo 2.0) (+ _teimpo 2.0)))
  (CallFunction|Sonido))

(event EventBeginPlay
  (bind _teimpo (Variables|Default|GetTeimpo))
  (Utilities|FlowControl|Delay (Math|Random|RandomFloatinRange (- _teimpo 2.0) (+ _teimpo 2.0)))
  (CallFunction|Sonido))

(fn ConstructionScript)