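; Unfinished light-flicker Blueprint, meant to vary the intensity of an owning Light actor.
; FlickTick resets its timer, waits briefly and compares it to TiempoActual before calling GetLightValues and StartFlick.
; GetLightValues randomizes a target intensity around the base and a new interval.
; BeginPlay is empty, light caching is disconnected, StartFlick's DoOnce drives nothing, and no intensity is ever applied.
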(event Custom|StartFlick
  (Utilities|FlowControl|DoOnce false))

(event Custom|FlickTick
  (Variables|Default|SetTiempoBase 0.0)
  (Utilities|FlowControl|Delay 0.2)
  (bind _output_get (Variables|Default|SetTiempoBase (+ (Variables|Default|GetTiempoBase) 0.2)))
  (if (>= _output_get (Variables|Default|GetTiempoActual))
    (CallFunction|GetLightValues)
    (CallFunction|StartFlick)))

(event EventBeginPlay)

(fn GetLightValues
  (bind _intensidadbase (Variables|Default|GetIntensidadBase))
  (bind _desviacionbase (Variables|Default|GetDesviacionBase))
  (Variables|Default|SetDesviacionActual (Math|Random|RandomFloatinRange (- _intensidadbase _desviacionbase) (+ _intensidadbase _desviacionbase)))
  (Variables|Default|SetTiempoActual (Math|Random|RandomFloatinRange 0.25 0.75)))