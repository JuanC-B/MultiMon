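; BP_Interactor is a one-shot orb trigger that hands activate by staying inside its sphere.
; Box component overlaps update a hand counter, growing the orb on entry and reversing the timeline when none remain.
; Completed growth disables it, calls Activate on each I_EventDependant in its Event array, then plays a closing scale animation and destroys the actor.
; Tick continuously spins the scene component through a multicast event.
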(event OnComponentBeginOverlap(Sphere)
  (params (OverlappedComponent :type Primitive%20Component%20Object%20Reference) (OtherActor :type Actor%20Object%20Reference) (OtherComp :type Primitive%20Component%20Object%20Reference) (OtherBodyIndex :type Integer) (bFromSweep :type Boolean) (SweepResult :type Hit%20Result%20Structure%20%28by%20ref%29))
  (Utilities|Casting|CastToBoxComponent OtherComp)
  (bind _result (Math|Integer|IncrementInt (Variables|Default|GetHandsInside))
    (:%20%20
      (if (> _result 0)
        (CallFunction|PlayAnimation)))))

(event OnComponentEndOverlap(Sphere)
  (params (OverlappedComponent :type Primitive%20Component%20Object%20Reference) (OtherActor :type Actor%20Object%20Reference) (OtherComp :type Primitive%20Component%20Object%20Reference) (OtherBodyIndex :type Integer))
  (Utilities|Casting|CastToBoxComponent OtherComp)
  (bind _result (Math|Integer|DecrementInt (Variables|Default|GetHandsInside))
    (:%20%20
      (if (<= _result 0)
        (CallFunction|ReverseAnimation)))))

(event Custom|PlayAnimation
  (if (Variables|Default|GetEnable)
    (Components|Timeline|SetPlayRate (Variables|Default|GetTL_orbIncrease) 3.0)
    (bind (_direction _alpha) (Timeline|TL_orbIncrease Play)
      (:Update
        (Transformation|SetRelativeScale3D (Variables|Default|GetOrb) (Math|Vector|MakeVector (Math|Float|Lerp 1.0 1.25 _alpha) (Math|Float|Lerp 1.0 1.25 _alpha) (Math|Float|Lerp 1.0 1.25 _alpha))))
      (:Finished
        (if (Utilities|Enum|Equal(Enum) _direction "Forward")
          (Variables|Default|SetEnable false)
          (for _array_element (Variables|Default|GetEvent)
            (bind _asi_event_dependant (Utilities|Casting|CastToI_EventDependant _array_element))
            (Default|Activate _asi_event_dependant))
          (Components|Timeline|SetPlayRate (Variables|Default|GetTL_CloseAnimation) 2.0)
          (bind _alpha_2 (Timeline|TL_CloseAnimation Play)
            (:Update
              (Transformation|SetActorScale3D (Math|Vector|MakeVector (Math|Float|Lerp 0.0 1.0 _alpha_2) (Math|Float|Lerp 0.0 1.0 _alpha_2) (Math|Float|Lerp 0.0 1.0 _alpha_2))))
            (:Finished
              (Actor|DestroyActor))))))))

(event Custom|ReverseAnimation
  (if (Variables|Default|GetEnable)
    (Components|Timeline|SetPlayRate (Variables|Default|GetTL_orbIncrease) 2.5)
    (bind (_direction _alpha) (Timeline|TL_orbIncrease Reverse)
      (:Update
        (Transformation|SetRelativeScale3D (Variables|Default|GetOrb) (Math|Vector|MakeVector (Math|Float|Lerp 1.0 1.25 _alpha) (Math|Float|Lerp 1.0 1.25 _alpha) (Math|Float|Lerp 1.0 1.25 _alpha))))
      (:Finished
        (if (Utilities|Enum|Equal(Enum) _direction "Forward")
          (Variables|Default|SetEnable false)
          (for _array_element (Variables|Default|GetEvent)
            (bind _asi_event_dependant (Utilities|Casting|CastToI_EventDependant _array_element))
            (Default|Activate _asi_event_dependant))
          (Components|Timeline|SetPlayRate (Variables|Default|GetTL_CloseAnimation) 2.0)
          (bind _alpha_2 (Timeline|TL_CloseAnimation Play)
            (:Update
              (Transformation|SetActorScale3D (Math|Vector|MakeVector (Math|Float|Lerp 0.0 1.0 _alpha_2) (Math|Float|Lerp 0.0 1.0 _alpha_2) (Math|Float|Lerp 0.0 1.0 _alpha_2))))
            (:Finished
              (Actor|DestroyActor))))))))

(event Custom|Tick
  (params (delta :type Float%20%28double-precision%29))
  (CallFunction|MulticastTick delta))

(event Custom|Multicast_tick
  (params (delta :type Float%20%28double-precision%29))
  (Transformation|AddRelativeRotation (Variables|Default|GetScene) (Math|Rotator|MakeRotator 0.0 0.0 (* delta 2e+02)) false false))

(event EventTick
  (params (DeltaSeconds :type Float%20%28single-precision%29))
  (CallFunction|Tick DeltaSeconds))

(fn ConstructionScript)