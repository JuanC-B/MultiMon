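; BP_lsDependant is an interaction Blueprint that gates a level sequence behind a required number of activations.
; Each Activate event increments Count, and reaching InputsNeed passes through a DoOnce so the payoff runs only once.
; After a fixed delay, it creates a player for the LS sequence, with no explicit Play call, then destroys every BP_Interactor in the level.
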(event EventActivate
  (bind _result (Math|Integer|IncrementInt (Variables|Default|Getcount))
    (:%20%20
      (if (>= _result (Variables|Default|GetInputsNeed))
        (Utilities|FlowControl|DoOnce false
          (:Completed
            (Utilities|FlowControl|Delay 14.0)
            (Sequencer|Player|CreateLevelSequencePlayer (Variables|Default|GetLS) (Variables|Default|GetSettings))
            (bind _outactors (Actor|GetAllActorsOfClass "/Game/Blueprints/Interaction/BP_Interactor.BP_Interactor_C"))
            (for _array_element _outactors
              (Actor|DestroyActor _array_element))))))))

(fn ConstructionScript)