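; Multiplayer name list that hands out entries from its Names array one after another.
; BeginPlay picks a random start index and sends it through a multicast event that sets CurrentIndex.
; GetName returns the name at that index and increments the local counter, wrapping by modulo, or reports invalid while the index is -1.
; The random roll has no authority check.
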(event Custom|InitialRandomIndex
  (CallFunction|MulticastSetValue (Math|Random|RandomIntegerinRange 0 (Utilities|Array|LastIndex (Variables|Default|GetNames)))))

(event Custom|Multicast_setValue
  (params (CurrentIndex :type Integer))
  (Variables|Default|SetCurrentIndex CurrentIndex))

(event EventBeginPlay
  (CallFunction|InitialRandomIndex))

(fn ConstructionScript)

(fn GetName
  (bind _names (Variables|Default|GetNames))
  (if (!= (Variables|Default|GetCurrentIndex) -1)
    (Math|Integer|IncrementInt (Variables|Default|GetCurrentIndex)
      (:%20%20
        (return (Utilities|Array|Get(acopy) _names (Math|Integer|%(Integer) (- (Variables|Default|GetCurrentIndex) 1) (Utilities|Array|Length _names))) true)))
    (else
      (return "" false))))