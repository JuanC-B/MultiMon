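; Matchmaking actor that automatically puts the player into a worldwide EIK online session shortly after BeginPlay, following three ping sounds.
; It searches "EikWorld" lobbies and joins the first populated one, only printing on success.
; If none is found or joining fails, it creates a lobby with voice chat and host migration, then opens EXTERIOR_MAP as listen server.
; Empty-session destruction and the time-based session-code hash are left unwired.
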(event Custom|WorldWide
  (bind _sessionresults (|FindEIKSessions (Utilities|Map|MakeMap "Lobby" (Utilities|Struct|MakeEIKAttribute "String" "EikWorld" false)) "MT_Lobby" 5 "RE_NoSelection" false false)
    (:OnSuccess
      (Development|PrintString (Utilities|String|Append "Success Find" (Utilities|String|ToString(Integer) (Utilities|Array|Length _sessionresults))))
      (bind _array_element (Utilities|Array|ForEachLoopwithBreak _sessionresults :!label _label)
        (:LoopBody
          (Development|PrintString (Utilities|String|Append "session  name:  " (.SessionName (Utilities|Struct|BreakSessionFindStruct _array_element)) " with " (Utilities|String|ToString(Integer) (.CurrentNumberOfPlayers (Utilities|Struct|BreakSessionFindStruct _array_element))) " players"))
          (if (> (.CurrentNumberOfPlayers (Utilities|Struct|BreakSessionFindStruct _array_element)) 0)
            (bind _output_get (Variables|Default|SetWWSessionToJoin _array_element))
            (Development|PrintString (Utilities|String|Append "new session to join:    " (.SessionName (Utilities|Struct|BreakSessionFindStruct _output_get)) " with " (Utilities|String|ToString(Integer) (.CurrentNumberOfPlayers (Utilities|Struct|BreakSessionFindStruct _output_get)))))
            (goto _label Break)
            (else
              (Development|PrintString (Utilities|String|Append "destroying: " (.SessionName (Utilities|Struct|BreakSessionFindStruct _array_element)))))))
        (:Completed
          (bind _returnvalue (Class|EIKBlueprintFunctions|IsValidSession (Variables|Default|GetWWSessionToJoin)))
          (if _returnvalue
            (Development|PrintString "FIND BRANCH TRUE")
            (|JoinEIKSessions (Utilities|String|StringToName (.SessionName (Utilities|Struct|BreakSessionFindStruct (Variables|Default|GetWWSessionToJoin)))) (Variables|Default|GetWWSessionToJoin) false
              (:OnSuccess
                (Development|PrintString (Utilities|String|Append "succes JOIN to:   " (.SessionName (Utilities|Struct|BreakSessionFindStruct (Variables|Default|GetWWSessionToJoin))))))
              (:OnFail
                (Development|PrintString "JOIN SESSION FAIL")
                (CallFunction|CreateNewServer :!label _label_2)))
            (else
              (Development|PrintString "FIND BRANCH FALSE")
              (goto _label_2))))))
    (:OnFail
      (Development|PrintString "Find Failure")
      (goto _label_2))))

(event Custom|CreateNewServer
  (Variables|Default|SetSessionCode (|SessionCodeHash_2_2))
  (|EIKLobby (Utilities|Map|MakeMap "Lobby" (Utilities|Struct|MakeEIKAttribute "String" "EikWorld" false)) (Utilities|String|StringToName (Utilities|String|Append "GameSession#" (Utilities|String|ToString(Integer) (Variables|Default|GetSessionCode)))) 3 (Utilities|Struct|MakeCreateLobbySettings false false 0 true true "RE_NoSelection" true false "" true true (Utilities|String|Append "GameSession#" (Utilities|String|ToString(Integer) (Variables|Default|GetSessionCode))))
    (:OnSuccess
      (Development|PrintString "CREATE LOBBY TRUE")
      (Game|OpenLevel(byObjectReference) "/Game/Maps/EXTERIOR_MAP.EXTERIOR_MAP" false "listen"))
    (:OnFail
      (Development|PrintString "CREATE LOBBY FAILURE")
      (Audio|PlaySound2D "/Engine/EditorSounds/Notifications/CompileFailed.CompileFailed" 1e+01 1.0 0.0 0 0))))

(event EventBeginPlay
  (Utilities|FlowControl|Delay 1.0)
  (Audio|PlaySound2D "/Engine/EngineSounds/1kSineTonePing.1kSineTonePing" 1.0 1.0 0.0 0 0)
  (Utilities|FlowControl|Delay 1.0)
  (Audio|PlaySound2D "/Engine/EngineSounds/1kSineTonePing.1kSineTonePing" 1.0 1.0 0.0 0 0)
  (Utilities|FlowControl|Delay 1.0)
  (Audio|PlaySound2D "/Engine/EngineSounds/1kSineTonePing.1kSineTonePing" 5.0 3.0 0.0 0 0)
  (CallFunction|WorldWide))

(event Collision|EventActorBeginOverlap
  (params (OtherActor :type Actor%20Object%20Reference)))

(event EventTick
  (params (DeltaSeconds :type Float%20%28single-precision%29)))

(fn ConstructionScript)